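; BP_TetrisBoard is a Tetris board Blueprint that owns the board data and keeps its line counter HUD current.
; The Construction Script creates an InternalBoard if none is valid, sized to the board width and height plus extra top space.
; On BeginPlay it binds to OnLinesCleared, and each clear passes the board to the WBP_BoardHUD in its LineCounter widget component to refresh the display.
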(event `self.ReceiveBeginPlay`
  ;[0 0 0] Bind gameplay delegates to components on BeginPlay
  (add `self.OnLinesCleared` (delegate `HandleOnLineCleared`)))

(event `HandleOnLineCleared`
  ;[0 0 0] Logic executed when lines are cleared
  (bind _aswbp_board_hud (cast `/Game/UMG/WBP_BoardHUD` (`WidgetComponent.GetWidget` (`self.LineCounter`))))
  (`BoardHUD.Update` _aswbp_board_hud self))

(fn `UserConstructionScript`
  ;[0 0 0] Initialize dependencies if they do not already exist.
  (`/Engine/EditorBlueprintResources/StandardMacros.IsValid` (`self.InternalBoard`)
    (:`Is Not Valid`
      (bind _returnvalue (`InternalBoard.NewInternalBoard` (`self.BoardWidth`) (+ (`self.BoardHeight`) (`self.BoardTopSpace`))))
      (set `self.InternalBoard` _returnvalue))))