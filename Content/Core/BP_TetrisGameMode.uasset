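; Game mode for a Tetris game that runs the start, game over and restart flow around the board actor.
; On BeginPlay it finds the BP_TetrisBoard, resets it and shows a start widget whose animation-finished event starts the game.
; The board's game over event opens a play-again widget that either quits or restores game input and re-enters the same reset-and-start sequence.
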(event `self.ReceiveBeginPlay`
  (`|ExecutionSequence`
    (:`then_0`
      ;[0 0 0] Register the Tetris board
      (bind _returnvalue (`GameplayStatics.GetActorOfClass` "/Game/Core/BP_TetrisBoard.BP_TetrisBoard_C"))
      (set `self.Board` _returnvalue))
    (:`then_1`
      ;[0 0 0] Events to execute on game over event
      (add `TetrisBoard.OnGameOver` (`self.Board`) (delegate `Create Game Over Widget`)))
    (:`then_2`
      (`TetrisBoard.Reset` (`self.Board`) :!label _label)
      (`KismetSystemLibrary.Delay` 0.5)
      (bind _returnvalue_2 (`|CreateWidget` "/Game/UMG/WBP_GameStart.WBP_GameStart_C" (`GameplayStatics.GetPlayerController` 0)))
      (bind _output_get (set `self.GameStartUI` _returnvalue_2))
      (add `/Game/UMG/WBP_GameStart.OnStartAnimationFinished` _output_get (delegate `Start Game`))
      (`UserWidget.AddToViewport` _output_get 0))))

(event `Create Game Over Widget`
  ;[0 0 0] Events to execute on game over event
  (bind _returnvalue (`|CreateWidget` "/Game/UMG/WBP_GameOver.WBP_GameOver_C" (`GameplayStatics.GetPlayerController` 0)))
  (bind _output_get (set `self.GameEndUI` _returnvalue))
  (add `/Game/UMG/WBP_GameOver.OnPlayAgainNo` _output_get (delegate `HandleOnPlayAgainNo`))
  (add `/Game/UMG/WBP_GameOver.OnPlayAgainYes` (`self.GameEndUI`) (delegate `HandleOnPlayAgainYes`))
  (`UserWidget.AddToViewport` (`self.GameEndUI`) 0))

(event `HandleOnPlayAgainNo`
  ;[0 0 0] Events to execute on game over event
  ;;[0 0 0] Quit game if no
  (`KismetSystemLibrary.QuitGame` null "Quit"))

(event `HandleOnPlayAgainYes`
  (bind _returnvalue (`GameplayStatics.GetPlayerController` 0))
  ;[0 0 0] Events to execute on game over event
  ;;[0 0 0] Restart game if yes
  (`Widget.RemoveFromParent` (`self.GameEndUI`))
  (set `PlayerController.bShowMouseCursor` false _returnvalue)
  (`WidgetBlueprintLibrary.SetInputMode_GameOnly` _returnvalue)
  (goto _label))

(event `Start Game`
  (`Widget.RemoveFromParent` (`self.GameStartUI`))
  (`TetrisBoard.StartGame` (`self.Board`)))

(fn `UserConstructionScript`)